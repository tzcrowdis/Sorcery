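; Enemy spawner that periodically spawns a randomly chosen melee or turret enemy around itself.
; BeginPlay starts two looping timers: one spawns at a random reachable navmesh point within SpawnRadius with random yaw, then randomizes elemental weakness.
; The other repeatedly halves SpawnRate, but never resets the spawn timer, so the actual interval stays at its initial value.
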(event Custom|Spawn%20Enemy
  (switch int (Math|Random|RandomIntegerinRange 0 1)
    (:0
      ;[1 1 1] Spawn Melee Enemy
      (bind _returnvalue (Game|SpawnActorfromClass "/Game/Enemies/MeleeEnemy/MeleeEnemy_BP.MeleeEnemy_BP_C" (Math|Transform|MakeTransform (.RandomLocation (AI|Navigation|GetRandomReachablePointinRadius (Transformation|GetActorLocation) (Variables|Default|GetSpawnRadius) 0 0)) (Math|Rotator|MakeRotator 0.0 0.0 (Math|Random|RandomFloatinRange 0.0 3.6e+02)) "1.000000,1.000000,1.000000") "AdjustIfPossibleButAlwaysSpawn" "MultiplyWithRoot" 0 0))
      (Utilities|IsValid _returnvalue
        (:Is%20Valid
          (Class|Enemy|RandomizeElementalWeakness _returnvalue))))
    (:1
      ;[1 1 1] Spawn Turret Enemy
      (bind _returnvalue_2 (Game|SpawnActorfromClass "/Game/Enemies/TurretEnemy/TurretEnemy_BP.TurretEnemy_BP_C" (Math|Transform|MakeTransform (.RandomLocation (AI|Navigation|GetRandomReachablePointinRadius (Transformation|GetActorLocation) (Variables|Default|GetSpawnRadius) 0 0)) (Math|Rotator|MakeRotator 0.0 0.0 (Math|Random|RandomFloatinRange 0.0 3.6e+02)) "1.000000,1.000000,1.000000") "AlwaysSpawn" "MultiplyWithRoot" 0 0))
      (Utilities|IsValid _returnvalue_2
        (:Is%20Valid
          (Class|Enemy|RandomizeElementalWeakness _returnvalue_2))))))

(event Custom|DecreaseSpawnRate
  ;[1 1 1] Every 2 minutes decrease spawn rate by 5%
  (Variables|Default|SetSpawnRate (* (Variables|Default|GetSpawnRate) 0.5)))

(event EventBeginPlay
  (Variables|Default|SetSpawnRate 5.0)
  (Utilities|Time|SetTimerbyEvent (delegate Custom|Spawn%20Enemy) (Variables|Default|GetSpawnRate) true)
  (Utilities|Time|SetTimerbyEvent (delegate Custom|DecreaseSpawnRate) 3e+01 true))

(fn ConstructionScript)