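; Enemy Blueprint that displays a health bar and floating damage numbers for an enemy.
; Tick sets the WB_EnemyHealthBar percent from health and turns the widget component toward the player camera.
; DrawFloatingDamageText passes the truncated absolute damage and weak-spot critical flag to that widget for display.
; A deprecated, unreachable alternative draws the text to a render target and feeds it through a dynamic material into a Niagara system at the impact point.
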(event EventBeginPlay)

(event Collision|EventActorBeginOverlap
  (params (OtherActor :type Actor%20Object%20Reference)))

(event EventTick
  (params (DeltaSeconds :type Float%20%28single-precision%29))
  (bind _health_bar_widget (Variables|Default|GetHealth%20Bar%20Widget))
  ;[1 1 1] Update Enemy Health Bar
  (bind _aswb_enemy_health_bar (Utilities|Casting|CastToWB_EnemyHealthBar (UserInterface|GetWidget (Variables|Default|GetHealth%20Bar%20Widget))))
  (Progress|SetPercent (Variables|/Game/Enemies/Widgets/WB_EnemyHealthBar.WB_EnemyHealthBar_C|GetHealthBar _aswb_enemy_health_bar) (/ (Variables|Default|GetHealth) (Variables|Default|GetMaxHealth)))
  ;[1 1 1] UI faces Camera
  (Transformation|SetWorldRotation _health_bar_widget (Math|Rotator|FindLookatRotation (Transformation|GetWorldLocation _health_bar_widget) (Transformation|GetWorldLocation (Variables|/Script/Engine.PlayerCameraManager|GetTransformComponent (Game|GetPlayerCameraManager 0)))) false false))

(event EventDrawFloatingDamageText
  (bind _aswb_enemy_health_bar (Utilities|Casting|CastToWB_EnemyHealthBar (UserInterface|GetWidget (Variables|Default|GetHealth%20Bar%20Widget))))
  (Variables|/Game/Enemies/Widgets/WB_EnemyHealthBar.WB_EnemyHealthBar_C|SetDamageString _aswb_enemy_health_bar (Utilities|String|SelectString (Utilities|String|ToString(Integer) (Math|Float|Truncate (Math|Float|Absolute(Float) (Variables|Default|GetDamageTaken)))) "" true))
  (Variables|/Game/Enemies/Widgets/WB_EnemyHealthBar.WB_EnemyHealthBar_C|SetCriticalHit _aswb_enemy_health_bar (Variables|Default|GetbWeakSpotHit))
  (Default|SetDamageText _aswb_enemy_health_bar))

(fn ConstructionScript)

(fn InitFloatingDamageData
  (Variables|FloatingDamage|SetFloatingDamageText (Utilities|String|SelectString (Utilities|String|ToString(Integer) (Math|Float|Truncate (Math|Float|Absolute(Float) (Variables|Default|GetDamageTaken)))) "" true))
  (Variables|FloatingDamage|SetFloatingDamageDimensions (Math|Vector2D|MakeVector2D (* (Math|Conversions|ToFloat(Integer) (Utilities|String|Len (Variables|FloatingDamage|GetFloatingDamageText))) 36.0) 36.0))
  (Variables|FloatingDamage|SetFloatingDamageOffset (/ (Variables|FloatingDamage|GetFloatingDamageDimensions) 2.0))
  (Variables|FloatingDamage|SetFloatingDamageTextColor (Math|Color|SelectColor "(R=1.000000,G=0.000000,B=0.000000,A=1.000000)" "(R=1.000000,G=1.000000,B=1.000000,A=1.000000)" (Variables|Default|GetbWeakSpotHit))))

(fn DrawFloatingDamage
  (bind _floatingdamagedimensions (Variables|FloatingDamage|GetFloatingDamageDimensions))
  (Utilities|FlowControl|Sequence
    (:then_0
      (Utilities|FlowControl|Sequence
        (:then_0
          (bind _returnvalue (Rendering|CreateRenderTarget2D (Math|Float|Truncate (.x _floatingdamagedimensions)) (Math|Float|Truncate (.y _floatingdamagedimensions)) "RTF_R8"))
          (Variables|FloatingDamage|SetTempFloatingDamageRT _returnvalue)
          (bind _returnvalue_2 (Rendering|Material|CreateDynamicMaterialInstance "/Game/Enemies/FloatingDamageText/M_FloatingDamage.M_FloatingDamage" "None" "None" :!class /Script/Engine.KismetMaterialLibrary))
          (Variables|FloatingDamage|SetFloatingDamageMaterial _returnvalue_2)
          (Rendering|Material|SetTextureParameterValue (Variables|FloatingDamage|GetFloatingDamageMaterial) "RT_FloatingDamage" (Variables|FloatingDamage|GetTempFloatingDamageRT)))
        (:then_1
          (bind (_canvas _size _context) (Rendering|BeginDrawCanvastoRenderTarget (Variables|FloatingDamage|GetTempFloatingDamageRT)))
          (Variables|FloatingDamage|SetTempCanvas _canvas)
          (Variables|FloatingDamage|SetTempCanvasContext _context)
          (HUD|DrawText (Variables|FloatingDamage|GetTempCanvas) "/Game/Enemies/FloatingDamageText/Garet-Book_Font.Garet-Book_Font" (Variables|FloatingDamage|GetFloatingDamageText) (Variables|FloatingDamage|GetFloatingDamageOffset) "(X=1.000000,Y=1.000000)" "(R=1.000000,G=1.000000,B=1.000000,A=1.000000)" 0.0 "(R=0.000000,G=0.000000,B=0.000000,A=1.000000)" "(X=1.000000,Y=1.000000)" true true false "(R=0.000000,G=0.000000,B=0.000000,A=1.000000)")
          (Rendering|EndDrawCanvastoRenderTarget (Variables|FloatingDamage|GetTempCanvasContext)))))
    (:then_1
      (Utilities|FlowControl|Sequence
        (:then_0
          (bind _returnvalue_3 (Niagara|SpawnSystematLocation "/Game/Enemies/FloatingDamageText/NS_FloatingDamage.NS_FloatingDamage" (Variables|Default|GetImpactPoint)))
          (Variables|FloatingDamage|SetTempFloatingDamageVFX _returnvalue_3))
        (:then_1
          (Niagara|SetNiagaraVariable(LinearColor) (Variables|FloatingDamage|GetTempFloatingDamageVFX) "FloatingDamageTextColor" (Variables|FloatingDamage|GetFloatingDamageTextColor))
          (Class|NiagaraComponent|SetVariableVec2 (Variables|FloatingDamage|GetTempFloatingDamageVFX) "FloatingDamageDimensions" (Variables|FloatingDamage|GetFloatingDamageDimensions))
          (Class|NiagaraComponent|SetVariableMaterial (Variables|FloatingDamage|GetTempFloatingDamageVFX) "FloatingDamageMaterial" (Variables|FloatingDamage|GetFloatingDamageMaterial)))))))