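; Melee enemy Blueprint that attacks the first-person player and shows a health bar with floating damage text.
; While in attack range, Tick turns it toward the player and uses Delays to pulse a damage sphere, skipping the initial wait on the first attack.
; The sphere's overlap deals placeholder damage, gated by a flag that resets after each pulse.
; A damage-text event updates the widget's health percentage, damage number and weak-spot critical flag.
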(event OnComponentBeginOverlap(DamageSphere)
  (params (OverlappedComponent :type Primitive%20Component%20Object%20Reference) (OtherActor :type Actor%20Object%20Reference) (OtherComp :type Primitive%20Component%20Object%20Reference) (OtherBodyIndex :type Integer) (bFromSweep :type Boolean) (SweepResult :type Hit%20Result%20Structure%20%28by%20ref%29))
  ;[1 1 1] Temporary melee attack
  (if (not (Variables|Default|GetDamageApplied))
    (bind _asbp_first_person_character (Utilities|Casting|CastToBP_FirstPersonCharacter OtherActor))
    (bind _returnvalue (Game|Damage|ApplyDamage _asbp_first_person_character 1e+01 0 0 "/Script/Engine.DamageType"))
    (Variables|Default|SetDamageApplied (>= _returnvalue 0.0))))

(event EventBeginPlay
  (bind _aswb_enemy_health_bar (Utilities|Casting|CastToWB_EnemyHealthBar (UserInterface|GetWidget (Variables|Default|GetHealthBar))))
  (Variables|Default|SetHealthBarWidget _aswb_enemy_health_bar)
  (Variables|Default|SetDamageApplied false)
  (Variables|Default|SetFirstAttack true))

(event EventTick
  (params (DeltaSeconds :type Float%20%28single-precision%29))
  (bind _damagesphere (Variables|Default|GetDamageSphere))
  (bind _damagesphere_2 (Variables|Default|GetDamageSphere))
  (bind _damagesphere_3 (Variables|Default|GetDamageSphere))
  ;[1 1 1] Temporary melee attack
  (if (Variables|Default|GetbInAttackRange)
    (Transformation|SetActorRotation (Math|Rotator|MakeRotator 0.0 0.0 (.Yaw (Math|Rotator|BreakRotator (Math|Rotator|FindLookatRotation (Transformation|GetActorLocation) (Transformation|GetActorLocation (Game|GetPlayerCharacter 0)))))))
    (if (Variables|Default|GetFirstAttack)
      (Variables|Default|SetFirstAttack false)
      (else
        (Utilities|FlowControl|Delay 2.0)))
    (Rendering|SetVisibility _damagesphere_2 true false)
    (Collision|SetCollisionEnabled _damagesphere_2 "QueryOnly")
    (Utilities|FlowControl|Delay 0.5)
    (Rendering|SetVisibility _damagesphere_3 false false)
    (Collision|SetCollisionEnabled _damagesphere_3 "NoCollision")
    (Variables|Default|SetDamageApplied false)
    (else
      (Class|MeleeEnemy|EndAttack)
      (Rendering|SetVisibility _damagesphere false false)
      (Collision|SetCollisionEnabled _damagesphere "NoCollision")
      (Variables|Default|SetFirstAttack true))))

(event EventDrawFloatingDamageText
  (bind _healthbarwidget (Variables|Default|GetHealthBarWidget))
  ;[1 1 1] Damage Text
  (Progress|SetPercent (Variables|/Game/Enemies/Widgets/WB_EnemyHealthBar.WB_EnemyHealthBar_C|GetHealthBar (Variables|Default|GetHealthBarWidget)) (/ (Variables|Default|GetHealth) (Variables|Default|GetMaxHealth)))
  (Variables|/Game/Enemies/Widgets/WB_EnemyHealthBar.WB_EnemyHealthBar_C|SetDamageString _healthbarwidget (Utilities|String|SelectString (Utilities|String|ToString(Integer) (Math|Float|Truncate (Math|Float|Absolute(Float) (Variables|Default|GetDamageTaken)))) "" true))
  (Variables|/Game/Enemies/Widgets/WB_EnemyHealthBar.WB_EnemyHealthBar_C|SetCriticalHit _healthbarwidget (Variables|Default|GetbWeakSpotHit))
  (Default|SetDamageText _healthbarwidget))

(fn ConstructionScript)