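; Spider enemy Blueprint with a randomized elemental weakness and visual feedback for hits.
; On BeginPlay it caches its health bar widget, rolls the weakness and stores the original body and weakspot materials.
; A damage text event updates the health bar and shows the damage amount, marking weakspot hits as critical.
; A flash event briefly swaps an element-specific emissive dynamic material onto either the weakspot or body mesh.
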(event EventBeginPlay
  (bind _aswb_enemy_health_bar (Utilities|Casting|CastToWB_EnemyHealthBar (UserInterface|GetWidget (Variables|Default|GetHealthBar))))
  (Variables|Default|SetHealthBarWidget _aswb_enemy_health_bar)
  (Class|Enemy|RandomizeElementalWeakness)
  (Variables|Default|SetInitialMaterial (Rendering|Material|GetMaterial (Variables|Character|GetMesh) 0))
  (Variables|Default|SetInitialWeakspotMaterial (Rendering|Material|GetMaterial (Variables|Default|GetElementalWeaknessMesh) 0)))

(event EventApplyDamageFlash
  (params (ElementType :type Damage%20Type%20Object%20Reference))
  (bind _bweakspothit (Variables|Default|GetbWeakSpotHit))
  ;[1 1 1] Damage Flash
  (bind _returnvalue (Class|Enemy|GetDamageFlashMaterial ElementType _bweakspothit))
  (bind _returnvalue_2 (Rendering|Material|CreateDynamicMaterialInstance _returnvalue "None" "None" :!class /Script/Engine.KismetMaterialLibrary))
  (Rendering|Material|SetScalarParameterValue _returnvalue_2 "EmissiveStrength" 5.0 :!class /Script/Engine.MaterialInstanceDynamic)
  (if _bweakspothit
    (Rendering|Material|SetMaterial (Variables|Default|GetElementalWeaknessMesh) 0 _returnvalue_2)
    (Utilities|FlowControl|Delay 0.1)
    (Rendering|Material|SetMaterial (Variables|Default|GetElementalWeaknessMesh) 0 (Variables|Default|GetInitialWeakspotMaterial))
    (else
      (Rendering|Material|SetMaterial (Variables|Character|GetMesh) 0 _returnvalue_2)
      (Utilities|FlowControl|Delay 0.1)
      (Rendering|Material|SetMaterial (Variables|Character|GetMesh) 0 (Variables|Default|GetInitialMaterial)))))

(event EventDrawFloatingDamageText
  (bind _healthbarwidget (Variables|Default|GetHealthBarWidget))
  ;[1 1 1] Damage Text
  (Progress|SetPercent (Variables|/Game/Enemies/Widgets/WB_EnemyHealthBar.WB_EnemyHealthBar_C|GetHealthBar (Variables|Default|GetHealthBarWidget)) (/ (Variables|Default|GetHealth) (Variables|Default|GetMaxHealth)))
  (Variables|/Game/Enemies/Widgets/WB_EnemyHealthBar.WB_EnemyHealthBar_C|SetDamageString _healthbarwidget (Utilities|String|SelectString (Utilities|String|ToString(Integer) (Math|Float|Truncate (Math|Float|Absolute(Float) (Variables|Default|GetDamageTaken)))) "" true))
  (Variables|/Game/Enemies/Widgets/WB_EnemyHealthBar.WB_EnemyHealthBar_C|SetCriticalHit _healthbarwidget (Variables|Default|GetbWeakSpotHit))
  (Default|SetDamageText _healthbarwidget))

(fn ConstructionScript)