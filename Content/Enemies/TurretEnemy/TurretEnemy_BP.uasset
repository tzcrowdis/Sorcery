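; Turret enemy that fires volleys of homing projectiles at targets in attack range and has a randomized elemental weakness.
; Tick drives the attack, with a short Delay pacing shots until the volley count is exceeded and a cooldown starts.
; Damage events update a health bar widget with damage text, play hit or death sounds, and briefly swap body or weakspot materials for an emissive flash chosen by element and critical hit.
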(event EventBeginPlay
  (bind _aswb_enemy_health_bar (Utilities|Casting|CastToWB_EnemyHealthBar (UserInterface|GetWidget (Variables|Default|GetHealthBar))))
  (Variables|Components|SetHealthBarWidget _aswb_enemy_health_bar)
  (Class|Enemy|RandomizeElementalWeakness)
  (Variables|Default|SetInitialMaterial (Rendering|Material|GetMaterial (Variables|Character|GetMesh) 0))
  (Variables|Default|SetInitialWeakspotMaterial (Rendering|Material|GetMaterial (Variables|Character|GetMesh) 1)))

(event EventApplyDamageFlash
  (params (ElementType :type Damage%20Type%20Object%20Reference))
  (bind _bweakspothit (Variables|Default|GetbWeakSpotHit))
  ;[1 1 1] Damage Flash
  (bind _returnvalue (Class|Enemy|GetDamageFlashMaterial ElementType _bweakspothit))
  (bind _returnvalue_2 (Rendering|Material|CreateDynamicMaterialInstance _returnvalue "None" "None" :!class /Script/Engine.KismetMaterialLibrary))
  (Rendering|Material|SetScalarParameterValue _returnvalue_2 "EmissiveStrength" 5.0 :!class /Script/Engine.MaterialInstanceDynamic)
  (if _bweakspothit
    (Rendering|Material|SetMaterial (Variables|Character|GetMesh) 1 _returnvalue_2)
    (Utilities|FlowControl|Delay 0.1)
    (Rendering|Material|SetMaterial (Variables|Character|GetMesh) 1 (Variables|Default|GetInitialWeakspotMaterial))
    (else
      (Rendering|Material|SetMaterial (Variables|Character|GetMesh) 0 _returnvalue_2)
      (Utilities|FlowControl|Delay 0.1)
      (Rendering|Material|SetMaterial (Variables|Character|GetMesh) 0 (Variables|Default|GetInitialMaterial)))))

(event EventPlayHitSound
  ;[1 1 1] Enemy Sounds
  (Audio|PlaySoundatLocation "/Game/Sorcery/Sounds/EnemyHitGrunt.EnemyHitGrunt" (Transformation|GetActorLocation) "0, 0, 0" 0.25 1.0 0.0 0 0 0 0))

(event EventDrawFloatingDamageText
  (bind _healthbarwidget (Variables|Components|GetHealthBarWidget))
  ;[1 1 1] Damage Text
  (Progress|SetPercent (Variables|/Game/Enemies/Widgets/WB_EnemyHealthBar.WB_EnemyHealthBar_C|GetHealthBar (Variables|Components|GetHealthBarWidget)) (/ (Variables|Default|GetHealth) (Variables|Default|GetMaxHealth)))
  (Variables|/Game/Enemies/Widgets/WB_EnemyHealthBar.WB_EnemyHealthBar_C|SetDamageString _healthbarwidget (Utilities|String|SelectString (Utilities|String|ToString(Integer) (Math|Float|Truncate (Math|Float|Absolute(Float) (Variables|Default|GetDamageTaken)))) "" true))
  (Variables|/Game/Enemies/Widgets/WB_EnemyHealthBar.WB_EnemyHealthBar_C|SetCriticalHit _healthbarwidget (Variables|Default|GetbWeakSpotHit))
  (Default|SetDamageText _healthbarwidget))

(event EventTick
  (params (DeltaSeconds :type Float%20%28single-precision%29))
  ;[1 1 1] Turret AI
  (if (and (Variables|Default|GetbInAttackRange) (not (Variables|Default|GetbShootCooldownActive)))
    (Utilities|FlowControl|Delay 0.2)
    (Class|TurretEnemy|SpawnHomingProjectile)
    (Math|Float|IncrementFloat (Variables|Default|GetVolleyIndex)
      (:%20%20
        (if (not (<= (Variables|Default|GetVolleyIndex) (Variables|Default|GetVolleyCount)))
          (Class|TurretEnemy|StartShootCooldown))))))

(event EventPlayDeathSound
  (bind _returnvalue (Transformation|GetActorLocation))
  ;[1 1 1] Enemy Sounds
  (Audio|PlaySoundatLocation "/Game/Sorcery/Sounds/EnemyDeathSparks.EnemyDeathSparks" _returnvalue "0, 0, 0" 0.5 1.0 0.0 0 0 0 0)
  (Audio|PlaySoundatLocation "/Game/Sorcery/Sounds/EnemyDeathScream.EnemyDeathScream" _returnvalue "0, 0, 0" 0.5 1.0 0.0 0 0 0 0))

(fn ConstructionScript)