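; BP_ChainLightning is an actor for a chain lightning modifier that propagates by spawning copies of itself onto other actors.
; SpawnChildLightning attaches each copy to its target, passes on breadth and damage with depth reduced by one, then applies it with damage type, element color and previous actor.
; DelayedDestroy removes the actor after a short delay.
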(event EventSpawnChildLightning
  (params (AttachToActor :type Actor%20Object%20Reference) (DamageType :type Object%20Class%20Reference) (ElementColor :type Linear%20Color%20Structure) (PreviousActor :type Actor%20Object%20Reference))
  (bind _returnvalue (Game|SpawnActorfromClass "BP_ChainLightning_C" (Math|Transform|MakeTransform "0, 0, 0" "0, 0, 0" "1.000000,1.000000,1.000000") "AlwaysSpawn" "MultiplyWithRoot" 0 0))
  (Transformation|AttachActorToActor _returnvalue AttachToActor "None" "SnapToTarget" "SnapToTarget" "KeepWorld" false)
  (Class|ChainLightning|SetChainLightningParams _returnvalue (Variables|Default|GetChainQuantityBreadth) (- (Variables|Default|GetChainQuantityDepth) 1) (Variables|Default|GetDamage))
  (Class|ChainLightning|ApplyChainLightning _returnvalue AttachToActor DamageType ElementColor PreviousActor))

(event EventDelayedDestroy
  (Utilities|FlowControl|Delay 0.4)
  (Actor|DestroyActor))

(fn ConstructionScript)