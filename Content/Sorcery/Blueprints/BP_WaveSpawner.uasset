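; Wave spawner actor that runs escalating enemy waves and shows wave count and intermission timer in a widget.
; A delayed recursive loop spawns melee or turret enemies at random reachable nearby points, scaling each wave's total by a multiplier.
; OnDestroyed bindings count kills; clearing a wave spawns a random upgrade and starts an intermission, which ends early if the upgrade is destroyed.
; UpgradeUnlock can replace the Chain Lightning unlock with its upgrades in the pool.
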(event Custom|StartWave
  (Utilities|Time|ClearandInvalidateTimerbyHandle (Variables|Default|GetWaveIntermissionTimer))
  (Default|CancelIntermissionTimer (Variables|Default|GetWaveSpawnerWidget))
  (Math|Integer|IncrementInt (Variables|Default|GetWave)
    (:%20%20
      (Default|SetWaveCount (Variables|Default|GetWaveSpawnerWidget) (Variables|Default|GetWave))
      (Variables|Default|SetEnemySpawnCount 0)
      (Variables|WaveVariables|SetMaxEnemySpawnCount (* (Variables|WaveVariables|GetMaxEnemySpawnCount) (Variables|WaveVariables|GetWaveSpawnCountMultiplier)))
      (Variables|Default|SetEnemyKillCount 0)
      (CallFunction|WaveSpawning))))

(event Custom|Spawn%20Enemy
  (switch int (Math|Random|RandomIntegerinRange 0 1)
    (:0
      ;[1 1 1] Spawn Melee Enemy
      (bind _returnvalue (Game|SpawnActorfromClass "/Game/Enemies/MeleeEnemy/MeleeEnemy_BP.MeleeEnemy_BP_C" (Math|Transform|MakeTransform (.RandomLocation (AI|Navigation|GetRandomReachablePointinRadius (Transformation|GetActorLocation) (Variables|Default|GetSpawnRadius) 0 0)) (Math|Rotator|MakeRotator 0.0 0.0 (Math|Random|RandomFloatinRange 0.0 3.6e+02)) "1.000000,1.000000,1.000000") "AdjustIfPossibleButAlwaysSpawn" "MultiplyWithRoot" 0 0))
      (Game|AssignOnDestroyed _returnvalue (delegate Custom|OnDestroyed_IncrementKillCount)))
    (:1
      ;[1 1 1] Spawn Turret Enemy
      (bind _returnvalue_2 (Game|SpawnActorfromClass "/Game/Enemies/TurretEnemy/TurretEnemy_BP.TurretEnemy_BP_C" (Math|Transform|MakeTransform (+ (.RandomLocation (AI|Navigation|GetRandomReachablePointinRadius (Transformation|GetActorLocation) (Variables|Default|GetSpawnRadius) 0 0)) "0.000000,0.000000,50.000000") (Math|Rotator|MakeRotator 0.0 0.0 (Math|Random|RandomFloatinRange 0.0 3.6e+02)) "1.000000,1.000000,1.000000") "AlwaysSpawn" "MultiplyWithRoot" 0 0))
      (Game|BindEventtoOnDestroyed _returnvalue_2 (delegate Custom|OnDestroyed_IncrementKillCount)))))

(event Custom|SpawnUpgrade
  (bind _upgradesarray (Variables|Default|GetUpgradesArray))
  (bind _outitem (Utilities|Array|Random _upgradesarray))
  (CallFunction|UpgradeUnlock _outitem)
  (bind _returnvalue (Game|SpawnActorfromClass _outitem (Math|Transform|MakeTransform (Transformation|GetActorLocation) "0, 0, 0" "1.000000,1.000000,1.000000") "AlwaysSpawn" "MultiplyWithRoot" 0 0))
  (Game|AssignOnDestroyed _returnvalue (delegate Custom|OnDestroyed_Event)))

(event Custom|EndWave
  (CallFunction|SpawnUpgrade)
  (bind _returnvalue (Utilities|Time|SetTimerbyEvent (delegate Custom|StartWave) (Variables|WaveVariables|GetIntermissionTime)))
  (bind _output_get (Variables|Default|SetWaveIntermissionTimer _returnvalue))
  (Default|SetIntermissionTimer (Variables|Default|GetWaveSpawnerWidget) _output_get))

(event Custom|OnDestroyed_IncrementKillCount
  (params (DestroyedActor :type Actor%20Object%20Reference))
  (Math|Integer|IncrementInt (Variables|Default|GetEnemyKillCount)))

(event Custom|OnDestroyed_Event
  (params (DestroyedActor :type Actor%20Object%20Reference))
  (CallFunction|StartWave))

(event Custom|WaveSpawning
  (if (< (Variables|Default|GetEnemySpawnCount) (Variables|WaveVariables|GetMaxEnemySpawnCount))
    (CallFunction|SpawnEnemy)
    (Math|Integer|IncrementInt (Variables|Default|GetEnemySpawnCount)
      (:%20%20
        _)))
  (if (>= (Variables|Default|GetEnemyKillCount) (Variables|WaveVariables|GetMaxEnemySpawnCount))
    (CallFunction|EndWave)
    (else
      (Utilities|FlowControl|Delay (Variables|WaveVariables|GetSpawnRate))
      (CallFunction|WaveSpawning))))

(event EventBeginPlay
  (bind _returnvalue (UserInterface|CreateWidget "/Game/Sorcery/UI/WB_WaveSpawnerUI.WB_WaveSpawnerUI_C" (Game|GetPlayerController 0)))
  (bind _output_get (Variables|Default|SetWaveSpawnerWidget _returnvalue))
  (UserInterface|Viewport|AddtoViewport _output_get 0)
  (Utilities|FlowControl|Delay 5.0)
  (CallFunction|StartWave))

(fn ConstructionScript)

(fn UpgradeUnlock
  (params (UnlockedUpgrade :type BP%20Upgrade%20Pickup%20Class%20Reference))
  (if (== UnlockedUpgrade "/Game/UpgradePickups/UpgradeVariants/BP_ChainLightningUnlock.BP_ChainLightningUnlock_C")
    ;[1 1 1] Switches Chain Lightning Unlock for its Upgrades once you have it
    (Utilities|Array|RemoveItem (Variables|Default|GetUpgradesArray) "/Game/UpgradePickups/UpgradeVariants/BP_ChainLightningUnlock.BP_ChainLightningUnlock_C")
    (Utilities|Array|AppendArray (Variables|Default|GetUpgradesArray) (Variables|Default|GetChainLightningUpgrades))))