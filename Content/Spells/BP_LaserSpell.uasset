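; BP_LaserSpell is a laser spell that deals damage at regular intervals while firing.
; Tick calls TickLaser while LaserFiring is set and keeps a looping timer running at AttackSpeed to call ApplyLaserDamage, clearing it when firing stops.
; UpdateReticle switches the player controller's SorceryCharacterWidget to the laser reticle.
; TickLaser and ApplyLaserDamage are called here but defined outside this graph.
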(event Custom|LaserDamageEvent
  ;[1 1 1] Ticks Damage at Regular Intervals
  (Class|LaserSpell|ApplyLaserDamage))

(event EventBeginPlay)

(event EventTick
  (params (DeltaSeconds :type Float%20%28single-precision%29))
  ;[1 1 1] Ticks Damage at Regular Intervals
  (if (Variables|Default|GetLaserFiring)
    (Class|LaserSpell|TickLaser)
    (if (not (Utilities|Time|IsTimerActivebyHandle (stale _returnvalue)))
      (bind _returnvalue (Utilities|Time|SetTimerbyEvent (delegate Custom|LaserDamageEvent) (Variables|Default|GetAttackSpeed) true)))
    (else
      (Utilities|Time|ClearandInvalidateTimerbyHandle _returnvalue))))

(event Collision|EventActorBeginOverlap
  (params (OtherActor :type Actor%20Object%20Reference)))

(event EventUpdateReticle
  ;[1 1 1] Changes the Reticle
  (bind _asbp_first_person_player_controller (Utilities|Casting|CastToBP_FirstPersonPlayerController (Game|GetPlayerController 0)))
  (Default|SetLaserReticle (Variables|/Game/Sorcery/Blueprints/BP_FirstPersonPlayerController.BP_FirstPersonPlayerController_C|GetSorceryCharacterWidget _asbp_first_person_player_controller)))

(fn ConstructionScript)