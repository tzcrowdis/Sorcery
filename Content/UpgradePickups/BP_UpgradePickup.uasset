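; Upgrade pickup Blueprint that handles the spawn and spin animation of its upgrade mesh, with no collection logic in its graphs.
; On BeginPlay a timeline drives the mesh's uniform world scale, then sets it to exactly one when finished.
; The UpgradeMeshMotion event plays or stops a second timeline that maps its track to world yaw in full turns, zeroing roll and pitch.
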(event EventBeginPlay
  (bind _scaletrack (Timeline|ScaleUpTimeline Play)
    (:Update
      (Transformation|SetWorldScale3D (Variables|Default|GetUpgradeMesh) (Math|Conversions|ToVector(Float) _scaletrack)))
    (:Finished
      (Transformation|SetWorldScale3D (Variables|Default|GetUpgradeMesh) (Class|KismetMathLibrary|VectorOne)))))

(event EventUpgradeMeshMotion
  (params (Enable :type Boolean))
  (if Enable
    (bind _rotationtrack (Timeline|RotationTimeline Play)
      (:Update
        (Transformation|SetWorldRotation (Variables|Default|GetUpgradeMesh) (Math|Rotator|MakeRotator 0.0 0.0 (* _rotationtrack 3.6e+02)) false false)))
    (else
      (Timeline|RotationTimeline Stop))))

(fn ConstructionScript)