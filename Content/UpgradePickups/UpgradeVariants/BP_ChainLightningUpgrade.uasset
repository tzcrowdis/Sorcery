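; Upgrade pickup variant that improves the Sorcerer's chain lightning.
; On BeginPlay it runs the parent setup, then sets the description text on its WB_UpgradeInfoMenu widget.
; ApplyUpgrade increments the Sorcerer's chain lightning depth and breadth and multiplies its damage by PercentChange.
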(event EventBeginPlay
  (|CallParentFunction)
  (bind _aswb_upgrade_info_menu (Utilities|Casting|CastToWB_UpgradeInfoMenu (UserInterface|GetUserWidgetObject (Variables|Default|GetInfoMenu))))
  (Default|SetDescriptionText _aswb_upgrade_info_menu "improve chain lightning."))

(event EventApplyUpgrade
  (params (Sorcerer :type Sorcery%20Character%20Object%20Reference))
  (Math|Integer|IncrementInt (Variables|/Script/Sorcery.SorceryCharacter|GetChainLightningDepth Sorcerer)
    (:%20%20
      (Math|Integer|IncrementInt (Variables|/Script/Sorcery.SorceryCharacter|GetChainLightningBreadth Sorcerer)
        (:%20%20
          (Variables|/Script/Sorcery.SorceryCharacter|SetChainLightningDamage Sorcerer (* (Variables|/Script/Sorcery.SorceryCharacter|GetChainLightningDamage Sorcerer) (Variables|Default|GetPercentChange))))))))

(fn ConstructionScript
  (|CallParentFunction))