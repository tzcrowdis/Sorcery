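; BP_DamageUpgrade is an upgrade pickup variant that raises a Sorcerer's spell damage.
; On BeginPlay it sets a five percent multiplier and writes its description into the pickup's info menu widget.
; When applied, it multiplies the Sorcerer's DamagePercent by that factor, so repeated upgrades compound, then refreshes the spell stats.
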(event EventBeginPlay
  (|CallParentFunction)
  (Variables|Default|SetPercentChange 1.05)
  (bind _aswb_upgrade_info_menu (Utilities|Casting|CastToWB_UpgradeInfoMenu (UserInterface|GetUserWidgetObject (Variables|Default|GetInfoMenu))))
  (Default|SetDescriptionText _aswb_upgrade_info_menu "Upgrades Damage"))

(event EventApplyUpgrade
  (params (Sorcerer :type Sorcery%20Character%20Object%20Reference))
  (Variables|/Script/Sorcery.SorceryCharacter|SetDamagePercent Sorcerer (* (Variables|/Script/Sorcery.SorceryCharacter|GetDamagePercent Sorcerer) (Variables|Default|GetPercentChange)))
  (Class|SorceryCharacter|UpdateSpellStats Sorcerer))

(fn ConstructionScript
  (|CallParentFunction))