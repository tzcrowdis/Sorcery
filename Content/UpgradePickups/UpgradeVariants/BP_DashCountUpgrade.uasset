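; Upgrade pickup variant that grants the Sorcerer an extra dash.
; On BeginPlay it runs the parent setup, then writes a dash-count description into the WB_UpgradeInfoMenu shown by its InfoMenu widget component.
; ApplyUpgrade increments the Sorcerer's DashMaxCount and calls UpdateDashCount to refresh it.
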(event EventBeginPlay
  (|CallParentFunction)
  (bind _aswb_upgrade_info_menu (Utilities|Casting|CastToWB_UpgradeInfoMenu (UserInterface|GetUserWidgetObject (Variables|Default|GetInfoMenu))))
  (Default|SetDescriptionText _aswb_upgrade_info_menu "Increases Number of Dashes"))

(event EventApplyUpgrade
  (params (Sorcerer :type Sorcery%20Character%20Object%20Reference))
  (Math|Integer|IncrementInt (Variables|/Script/Sorcery.SorceryCharacter|GetDashMaxCount Sorcerer)
    (:%20%20
      (Class|SorceryCharacter|UpdateDashCount Sorcerer))))

(fn ConstructionScript
  (|CallParentFunction))