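; Upgrade pickup variant that increases the Sorcerer's dash distance by scaling its dash velocity.
; On BeginPlay it runs the parent logic, then sets the description text on its InfoMenu's WB_UpgradeInfoMenu widget.
; ApplyUpgrade multiplies the Sorcerer's DashVelocity by PercentChange, so the value acts as a direct multiplier and repeated applications compound.
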(event EventBeginPlay
  (|CallParentFunction)
  (bind _aswb_upgrade_info_menu (Utilities|Casting|CastToWB_UpgradeInfoMenu (UserInterface|GetUserWidgetObject (Variables|Default|GetInfoMenu))))
  (Default|SetDescriptionText _aswb_upgrade_info_menu "increase dash distance."))

(event EventApplyUpgrade
  (params (Sorcerer :type Sorcery%20Character%20Object%20Reference))
  (Variables|/Script/Sorcery.SorceryCharacter|SetDashVelocity Sorcerer (* (Variables|/Script/Sorcery.SorceryCharacter|GetDashVelocity Sorcerer) (Variables|Default|GetPercentChange))))

(fn ConstructionScript
  (|CallParentFunction))