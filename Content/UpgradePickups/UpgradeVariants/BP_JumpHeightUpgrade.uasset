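; Upgrade pickup variant that raises the Sorcerer's jump height when applied.
; On BeginPlay it runs the parent setup, sets a small percentage multiplier and writes its description into the InfoMenu's upgrade info widget.
; ApplyUpgrade multiplies the Sorcerer's CharacterMovement JumpZVelocity by that multiplier, so repeated applications compound.
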(event EventBeginPlay
  (|CallParentFunction)
  (Variables|Default|SetPercentChange 1.05)
  (bind _aswb_upgrade_info_menu (Utilities|Casting|CastToWB_UpgradeInfoMenu (UserInterface|GetUserWidgetObject (Variables|Default|GetInfoMenu))))
  (Default|SetDescriptionText _aswb_upgrade_info_menu "Upgrades Jump Height"))

(event EventApplyUpgrade
  (params (Sorcerer :type Sorcery%20Character%20Object%20Reference))
  (bind _charactermovement (Variables|/Script/Engine.Character|GetCharacterMovement Sorcerer))
  (Variables|/Script/Engine.CharacterMovementComponent|SetJumpZVelocity _charactermovement (* (Variables|/Script/Engine.CharacterMovementComponent|GetJumpZVelocity _charactermovement) (Variables|Default|GetPercentChange))))

(fn ConstructionScript
  (|CallParentFunction))