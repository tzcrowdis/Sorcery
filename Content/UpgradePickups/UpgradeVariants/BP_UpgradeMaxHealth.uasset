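; Upgrade pickup variant that raises a Sorcerer's maximum health.
; On BeginPlay it runs the parent logic, sets a five percent increase multiplier and writes its description into the info menu widget.
; ApplyUpgrade multiplies the Sorcerer's MaxHealth by that multiplier, then refreshes the health bar through the first-person player controller's character widget.
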(event EventBeginPlay
  (|CallParentFunction)
  (Variables|Default|SetPercentChange 1.05)
  (bind _aswb_upgrade_info_menu (Utilities|Casting|CastToWB_UpgradeInfoMenu (UserInterface|GetUserWidgetObject (Variables|Default|GetInfoMenu))))
  (Default|SetDescriptionText _aswb_upgrade_info_menu "Upgrades Max Health"))

(event EventApplyUpgrade
  (params (Sorcerer :type Sorcery%20Character%20Object%20Reference))
  (Variables|/Script/Sorcery.SorceryCharacter|SetMaxHealth Sorcerer (* (Variables|/Script/Sorcery.SorceryCharacter|GetMaxHealth Sorcerer) (Variables|Default|GetPercentChange)))
  (bind _asbp_first_person_player_controller (Utilities|Casting|CastToBP_FirstPersonPlayerController (Pawn|GetController Sorcerer)))
  (Default|UpdateHealthBar (Variables|/Game/Sorcery/Blueprints/BP_FirstPersonPlayerController.BP_FirstPersonPlayerController_C|GetSorceryCharacterWidget _asbp_first_person_player_controller) false))

(fn ConstructionScript
  (|CallParentFunction))